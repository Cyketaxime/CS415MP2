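; Stompable enemy Blueprint that hurts the learning-kit player character on body contact, then self-destructs after a delay.
; A hit on Head bounces the player up and destroys the enemy immediately.
; A hit on BoxCol deals light damage, triggers the player's hit reaction, then after a delay spawns an emitter, heavily damages that player if player 0 is nearby, and destroys itself.
; A ScoreChange call is left unconnected.
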(event `self.Head.OnComponentHit`
  (params (HitComponent :type "PrimitiveComponent Object Reference") (OtherActor :type "Actor Object Reference") (OtherComp :type "PrimitiveComponent Object Reference") (NormalImpulse :type "Vector Structure") (Hit :type "HitResult Structure (by ref)"))
  (bind _asbp_learning_kit_player_character (cast `/Game/LearningKit_Games/Blueprints/PlayerCharacter/BP_LearningKit_PlayerCharacter` OtherActor))
  (`/Game/LearningKit_Games/Blueprints/PlayerCharacter/BP_LearningKit_PlayerCharacter.BounceUp` _asbp_learning_kit_player_character)
  (`self.K2_DestroyActor`))

(event `self.BoxCol.OnComponentHit`
  (params (HitComponent :type "PrimitiveComponent Object Reference") (OtherActor :type "Actor Object Reference") (OtherComp :type "PrimitiveComponent Object Reference") (NormalImpulse :type "Vector Structure") (Hit :type "HitResult Structure (by ref)"))
  (bind _asbp_learning_kit_player_character (cast `/Game/LearningKit_Games/Blueprints/PlayerCharacter/BP_LearningKit_PlayerCharacter` OtherActor))
  (`GameplayStatics.ApplyDamage` _asbp_learning_kit_player_character 1.0)
  (`/Game/LearningKit_Games/Blueprints/PlayerCharacter/BP_LearningKit_PlayerCharacter.WhenHit` _asbp_learning_kit_player_character (`self.K2_GetActorLocation` self))
  (`KismetSystemLibrary.Delay` 5.0)
  (`GameplayStatics.SpawnEmitterAtLocation` null (`self.K2_GetActorLocation` self) (struct) (3.0 3.0 3.0))
  (if (<= (`self.GetDistanceTo` (`GameplayStatics.GetPlayerCharacter` 0)) 500.0)
    (`GameplayStatics.ApplyDamage` _asbp_learning_kit_player_character 30.0))
  (`self.K2_DestroyActor`))

(fn `UserConstructionScript`)