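; BP_MortarProjectile is a short-lived mortar projectile that damages the Learning Kit player character on contact.
; It sets a brief lifespan on BeginPlay and relies on its SphereColl component for contact events.
; Any overlap spawns a scaled-up emitter and destroys the actor, first applying damage and calling WhenHit with its location if the player was struck.
; A blocking hit destroys it without effect or damage.
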(event `self.ReceiveBeginPlay`
  (`self.SetLifeSpan` 2.0))

(event `self.SphereColl.OnComponentBeginOverlap`
  (params (OverlappedComponent :type "PrimitiveComponent Object Reference") (OtherActor :type "Actor Object Reference") (OtherComp :type "PrimitiveComponent Object Reference") (OtherBodyIndex :type Integer) (bFromSweep :type Boolean) (SweepResult :type "HitResult Structure (by ref)"))
  (`GameplayStatics.SpawnEmitterAtLocation` null (`self.K2_GetActorLocation` self) (struct) (3.0 3.0 3.0))
  (bind _asbp_learning_kit_player_character (cast `/Game/LearningKit_Games/Blueprints/PlayerCharacter/BP_LearningKit_PlayerCharacter` OtherActor)
    (:`then`
      (`GameplayStatics.ApplyDamage` _asbp_learning_kit_player_character 5.0)
      (`/Game/LearningKit_Games/Blueprints/PlayerCharacter/BP_LearningKit_PlayerCharacter.WhenHit` _asbp_learning_kit_player_character (`self.K2_GetActorLocation` self))
      (`self.K2_DestroyActor`))
    (:`CastFailed`
      (`self.K2_DestroyActor`))))

(event `self.SphereColl.OnComponentHit`
  (params (HitComponent :type "PrimitiveComponent Object Reference") (OtherActor :type "Actor Object Reference") (OtherComp :type "PrimitiveComponent Object Reference") (NormalImpulse :type "Vector Structure") (Hit :type "HitResult Structure (by ref)"))
  (`self.K2_DestroyActor`))

(fn `UserConstructionScript`)