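; BP_Mortar is a stationary hazard that fires projectiles and can be destroyed by the player hitting its head.
; A looping timer, its interval randomized once at BeginPlay, spawns BP_MortarProjectile at the Arrow component's transform.
; Player contact with Head bounces the player and destroys the mortar, while Body contact applies damage and calls WhenHit with the mortar's location.
; A ScoreChange call is left unconnected.
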(event `self.ReceiveBeginPlay`
  (`KismetSystemLibrary.K2_SetTimer` null "LaunchProjectile" (`KismetMathLibrary.RandomFloatInRange` 2.0 5.0) true))

(event `self.Head.OnComponentHit`
  (params (HitComponent :type "PrimitiveComponent Object Reference") (OtherActor :type "Actor Object Reference") (OtherComp :type "PrimitiveComponent Object Reference") (NormalImpulse :type "Vector Structure") (Hit :type "HitResult Structure (by ref)"))
  (bind _asbp_learning_kit_player_character (cast `/Game/LearningKit_Games/Blueprints/PlayerCharacter/BP_LearningKit_PlayerCharacter` OtherActor))
  (`/Game/LearningKit_Games/Blueprints/PlayerCharacter/BP_LearningKit_PlayerCharacter.BounceUp` _asbp_learning_kit_player_character)
  (`self.K2_DestroyActor`))

(event `self.Body.OnComponentHit`
  (params (HitComponent :type "PrimitiveComponent Object Reference") (OtherActor :type "Actor Object Reference") (OtherComp :type "PrimitiveComponent Object Reference") (NormalImpulse :type "Vector Structure") (Hit :type "HitResult Structure (by ref)"))
  (bind _asbp_learning_kit_player_character (cast `/Game/LearningKit_Games/Blueprints/PlayerCharacter/BP_LearningKit_PlayerCharacter` OtherActor))
  (`GameplayStatics.ApplyDamage` _asbp_learning_kit_player_character 5.0)
  (`/Game/LearningKit_Games/Blueprints/PlayerCharacter/BP_LearningKit_PlayerCharacter.WhenHit` _asbp_learning_kit_player_character (`self.K2_GetActorLocation` self)))

(fn `LaunchProjectile`
  (bind _arrow (`self.Arrow`))
  (`|SpawnActorFromClass` "/Game/LearningKit_Games/Blueprints/BaseClasses/BP_MortarProjectile.BP_MortarProjectile_C" (`KismetMathLibrary.MakeTransform` (`SceneComponent.K2_GetComponentLocation` _arrow) (`SceneComponent.K2_GetComponentRotation` _arrow)) "Undefined" "MultiplyWithRoot" null null))

(fn `UserConstructionScript`)